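; BP_Map is a map actor in the MiniMap folder that pans horizontally while the left mouse button is held.
; Tick runs the Rotator Weapon graph, which calls Vector while TumbleActive is set.
; Vector scales input-axis values, passes them through TransformLocation and teleports the actor by the X/Y result.
; Despite the weapon-rotation names, the yaw rotate and timeline-driven ease functions sit only on never-run paths.
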(event Custom|RotatorWeapon
  (|RotatorWeapon))

(event EventBeginPlay)

(event Collision|EventActorBeginOverlap
  (params (OtherActor :type Actor%20Object%20Reference)))

(event EventTick
  (params (DeltaSeconds :type Float%20%28single-precision%29))
  (CallFunction|RotatorWeapon))

(fn ConstructionScript)

(fn RotateWeaponon
  (bind _defaultsceneroot (Variables|Default|GetDefaultSceneRoot))
  (bind _output_get (Variables|Default|SetRotator (Math|Rotator|CombineRotators (Transformation|GetWorldRotation _defaultsceneroot) (Math|Rotator|MakeRotator 0.0 0.0 (* (* (Class|Actor|GetInputAxisKeyValue) -1.0) (Variables|Default|GetTuvbleSpeed))))))
  (Transformation|SetWorldRotation _defaultsceneroot _output_get false false))

(fn RotateWeaponOff
  (params (InterpSpeed :type Float%20%28single-precision%29))
  (bind _output_get (Variables|Default|SetRotator (Math|Rotator|MakeRotator 0.0 0.0 (Math|Interpolation|FInterpTo (.yaw (Variables|Default|GetRotator)) 0.0 (Utilities|Time|GetWorldDeltaSeconds) InterpSpeed))))
  (Transformation|SetWorldRotation (Variables|Default|GetDefaultSceneRoot) (Math|Rotator|MakeRotator (.roll _output_get) (.pitch _output_get) (.yaw _output_get)) false false))

(fn Vector
  (bind _returnvalue (Class|Actor|GetInputAxisKeyValue))
  (bind _returnvalue_2 (Class|Actor|GetInputAxisKeyValue))
  (bind _newvar_0 (Variables|Default|GetNewVar_0))
  (bind _newvar_0_2 (Variables|Default|GetNewVar_0))
  (bind _returnvalue_3 (* _returnvalue _newvar_0))
  (bind _returnvalue_4 (* _returnvalue_2 -1.0))
  (bind _returnvalue_5 (* _returnvalue_4 _newvar_0_2))
  (bind _returnvalue_6 (Math|Transform|TransformLocation (Math|Transform|MakeTransform (Math|Vector|MakeVector _returnvalue_3 _returnvalue_5 0.0) "0, 0, 0" "1,1,1") (Math|Vector|MakeVector 0.0 0.0 0.0)))
  (Transformation|SetActorLocation self (+ (Transformation|GetActorLocation) (Math|Vector|MakeVector (.x _returnvalue_6) (.y _returnvalue_6) 0.0)) false true))

(event Input|MouseEvents|LeftMouseButton
  (params (Key :type Key%20Structure :default "None"))
  (:Pressed
    (Variables|Default|SetTumbleActive true))
  (:Released
    (Variables|Default|SetTumbleActive false)))