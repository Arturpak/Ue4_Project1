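; BP_MyFunctions is a Blueprint helper library of shortcuts to the game's framework objects.
; Getters fetch the game instance and player 0's character, controller or HUD, cast to the project classes for default gameplay, main menu and map contexts.
; The main menu controller and HUD getters use the Weapon-named classes, and a failed cast returns nothing.
; A Print Text helper wraps PrintString with color and duration.
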(fn DefaultCharacter
  (bind _asbp_player_character (Utilities|Casting|CastToBP_PlayerCharacter (Game|GetPlayerCharacter 0)))
  (return _asbp_player_character))

(fn DefaultHUD
  (bind _asbp_hud (Utilities|Casting|CastToBP_HUD (HUD|GetHUD (Game|GetPlayerController 0))))
  (return _asbp_hud))

(fn GameInstance
  (bind _asbp_game_instance (Utilities|Casting|CastToBP_GameInstance (Game|GetGameInstance)))
  (return _asbp_game_instance))

(fn MainMenuCharacter
  (bind _asbp_character_menu (Utilities|Casting|CastToBP_CharacterMenu (Game|GetPlayerCharacter 0)))
  (return _asbp_character_menu))

(fn MainMenuPlayerController
  (bind _asbp_player_controller_weapon (Utilities|Casting|CastToBP_PlayerControllerWeapon (Game|GetPlayerController 0)))
  (return _asbp_player_controller_weapon))

(fn MainMenuHUD
  (bind _asbp_hud_weapon (Utilities|Casting|CastToBP_HUD_Weapon (HUD|GetHUD (Game|GetPlayerController 0))))
  (return _asbp_hud_weapon))

(fn PrintText
  (params (Tex :type String) (Color :type Linear%20Color%20Structure :default "(R=0.572917,G=0.434809,B=0.149576,A=1.000000)") (Duration :type Float%20%28single-precision%29))
  (Development|PrintString 0 Tex true true Color Duration))

(fn ControllerMap
  (bind _asbp_map_controller (Utilities|Casting|CastToBP_MapController (Game|GetPlayerController 0)))
  (return _asbp_map_controller))

(fn DefaultPlayerController
  (bind _asbp_player_controller (Utilities|Casting|CastToBP_PlayerController (Game|GetPlayerController 0)))
  (return _asbp_player_controller))

(fn CharacterMap
  (bind _asbp_character_map (Utilities|Casting|CastToBP_CharacterMap (Game|GetPlayerCharacter 0)))
  (return _asbp_character_map))