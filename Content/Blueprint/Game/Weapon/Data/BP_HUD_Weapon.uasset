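; HUD Blueprint for the weapon menus that shows the mouse cursor and opens the main menu on BeginPlay.
; Display functions create or remove widgets for the main menu, weapon customization, inventory collection and weapon modules.
; Customization, collection and module functions toggle on widget validity, whatever Boolean is passed.
; DisplayMarkerModule and DisplayHUD create widgets without adding them to the viewport, and both remove the marker widget.
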(event EventBeginPlay
  (Variables|/Script/Engine.PlayerController|SetbShowMouseCursor (Game|GetPlayerController 0) true)
  (CallFunction|DisplayMainMenu true))

(fn ConstructionScript)

(fn DisplayMarkerModule
  (params (Visible :type Boolean))
  (bind _output_get (Variables|Default|SetMarkerModule? Visible))
  (if _output_get
    (Utilities|IsValid (Variables|Widget|GetW_MarkerModule)
      (:Is%20Valid
        (Widget|RemovefromParent (Variables|Widget|GetW_MarkerModule) :!label _label)
        (Variables|Widget|SetW_MarkerModule 0))
      (:Is%20Not%20Valid
        (bind _returnvalue (UserInterface|CreateWidget "/Game/Blueprint/Game/Weapon/Data/Interface/W_MarkerModule.W_MarkerModule_C" (CallFunction|MainMenuPlayerController)))
        (bind _output_get_2 (Variables|Widget|SetW_MarkerModule _returnvalue))
        (Input|SetInputModeGameandUI (Game|GetPlayerController 0) _output_get_2 "LockOnCapture" false)))
    (else
      (Utilities|IsValid (Variables|Widget|GetW_MarkerModule)
        (:Is%20Valid
          (goto _label))))))

(fn DisplayWeaponCustomization
  (params (Condition :type Boolean))
  (bind _output_get (Variables|Default|SetWeaponCustomization? Condition))
  (if _output_get
    (Utilities|IsValid (Variables|Widget|GetW_WeaponMenu)
      (:Is%20Valid
        (Widget|RemovefromParent (Variables|Widget|GetW_WeaponMenu) :!label _label)
        (Variables|Widget|SetW_WeaponMenu 0))
      (:Is%20Not%20Valid
        (bind _returnvalue (UserInterface|CreateWidget "/Game/Blueprint/Interface/WeaponMenu/W_WeaponMenu.W_WeaponMenu_C" (CallFunction|MainMenuPlayerController) :!label _label_2))
        (bind _output_get_2 (Variables|Widget|SetW_WeaponMenu _returnvalue))
        (UserInterface|Viewport|AddtoViewport _output_get_2 0)))
    (else
      (Utilities|IsValid (Variables|Widget|GetW_WeaponMenu)
        (:Is%20Valid
          (goto _label))
        (:Is%20Not%20Valid
          (goto _label_2))))))

(fn DisplayHUD
  (params (Visible :type Boolean))
  (bind _output_get (Variables|Default|SetHUD? Visible))
  (if _output_get
    (Utilities|IsValid (Variables|Widget|GetW_MarkerModule)
      (:Is%20Valid
        (Widget|RemovefromParent (Variables|Widget|GetW_MarkerModule) :!label _label)
        (Variables|Widget|SetW_MarkerModule 0))
      (:Is%20Not%20Valid
        (UserInterface|CreateWidget "/Game/Blueprint/Interface/WeaponMenu/W_InventoryMenu.W_InventoryMenu_C" (CallFunction|MainMenuPlayerController))))
    (else
      (Utilities|IsValid (Variables|Widget|GetW_MarkerModule)
        (:Is%20Valid
          (goto _label))))))

(fn DisplayMainMenu
  (params (Condition :type Boolean))
  (bind _output_get (Variables|Default|SetMainMenu? Condition))
  (if _output_get
    (bind _returnvalue (UserInterface|CreateWidget "/Game/Blueprint/Interface/MainMenu/W_MainMenu.W_MainMenu_C" (CallFunction|MainMenuPlayerController)))
    (bind _output_get_2 (Variables|Widget|SetW_MainMenu _returnvalue))
    (UserInterface|Viewport|AddtoViewport _output_get_2 0)
    (else
      (Widget|RemovefromParent (Variables|Widget|GetW_MainMenu)))))

(fn DisplayCollection
  (params (Condition :type Boolean))
  (bind _output_get (Variables|Default|SetCollection? Condition))
  (if _output_get
    (Utilities|IsValid (Variables|Default|GetW_Collection)
      (:Is%20Valid
        (Widget|RemovefromParent (Variables|Default|GetW_Collection) :!label _label)
        (Variables|Default|SetW_Collection 0))
      (:Is%20Not%20Valid
        (bind _returnvalue (UserInterface|CreateWidget "/Game/Blueprint/Interface/WeaponMenu/W_InventoryMenu.W_InventoryMenu_C" (CallFunction|MainMenuPlayerController) :!label _label_2))
        (bind _output_get_2 (Variables|Default|SetW_Collection _returnvalue))
        (UserInterface|Viewport|AddtoViewport _output_get_2 0)))
    (else
      (Utilities|IsValid (Variables|Default|GetW_Collection)
        (:Is%20Valid
          (goto _label))
        (:Is%20Not%20Valid
          (goto _label_2))))))

(fn DisplayCurrentModule
  (params (Condition :type Boolean))
  (bind _output_get (Variables|Default|SetModule? Condition))
  (if _output_get
    (Utilities|IsValid (Variables|Default|GetW_WeaponModule)
      (:Is%20Valid
        (Widget|RemovefromParent (Variables|Default|GetW_WeaponModule) :!label _label)
        (Variables|Default|SetW_WeaponModule 0))
      (:Is%20Not%20Valid
        (bind _returnvalue (UserInterface|CreateWidget "/Game/Blueprint/Interface/WeaponMenu/W_WeaponModule.W_WeaponModule_C" (CallFunction|MainMenuPlayerController) :!label _label_2))
        (bind _output_get_2 (Variables|Default|SetW_WeaponModule _returnvalue))
        (UserInterface|Viewport|AddtoViewport _output_get_2 0)))
    (else
      (Utilities|IsValid (Variables|Default|GetW_WeaponModule)
        (:Is%20Valid
          (goto _label))
        (:Is%20Not%20Valid
          (goto _label_2))))))

(fn DisplayCurrentModule2222
  (params (Condition :type Boolean))
  (if Condition
    (Utilities|IsValid (Variables|Default|GetW_SLotModule)
      (:Is%20Valid
        (Widget|RemovefromParent (Variables|Default|GetW_SLotModule) :!label _label)
        (Variables|Default|SetW_SLotModule 0))
      (:Is%20Not%20Valid
        (bind _returnvalue (UserInterface|CreateWidget "/Game/Blueprint/Interface/WeaponMenu/W_WeaponModule1.W_WeaponModule1_C" (CallFunction|MainMenuPlayerController) :!label _label_2))
        (bind _output_get (Variables|Default|SetW_SLotModule _returnvalue))
        (UserInterface|Viewport|AddtoViewport _output_get 0)))
    (else
      (Utilities|IsValid (Variables|Default|GetW_SLotModule)
        (:Is%20Valid
          (goto _label))
        (:Is%20Not%20Valid
          (goto _label_2))))))