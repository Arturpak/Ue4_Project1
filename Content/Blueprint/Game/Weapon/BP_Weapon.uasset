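; BP_Weapon is a weapon Blueprint that handles ammo consumption and fire-rate limiting, with no projectile or damage logic of its own.
; UseWeapon spends one ammo when able, returns whether it succeeded, and starts a timer that blocks further use for UseRate.
; With AutoFire, the timer callback StopRateDealy fires again until StopUseWeapon clears FireActive or an attempt fails.
; The construction script calls CurrentModules, which is empty.
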(fn ConstructionScript
  (CallFunction|CurrentModules))

(fn CurrentModules
  (return))

(fn UseWeapon
  (if (CallFunction|AbletoUseWeapon)
    (Math|Integer|DecrementInt (Variables|Default|GetCurrentAmmo)
      (:%20%20
        (Utilities|Time|SetTimerbyFunctionName 0 "StopRateDealy" (Variables|Default|GetUseRate))
        (Variables|Default|SetUseFreezedByRate true)
        (if (Variables|Default|GetAutoFire)
          (Variables|Default|SetFireActive true))
        (return true)))
    (else
      (Variables|Default|SetFireActive false)
      (return false))))

(fn AbletoUseWeapon
  (return (and (not (Variables|Default|GetUseFreezedByRate)) (> (Variables|Default|GetCurrentAmmo) 0))))

(fn StopRateDealy
  (Variables|Default|SetUseFreezedByRate false)
  (if (and (Variables|Default|GetAutoFire) (Variables|Default|GetFireActive))
    (CallFunction|UseWeapon)))

(fn StopUseWeapon
  (Variables|Default|SetFireActive false))