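; BP_EnemyCharacter is an AI enemy Character that loses health when hit and dies at zero HP.
; Capsule hits from actors passing a cast subtract fixed damage; at zero HP the capsule starts simulating physics, then the actor is destroyed after a delay.
; SetSpeed scales walk speed from DefaultSpeed, and Tick prints HP for debugging.
; An attached particle emitter spawn for hits exists but never runs.
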(event OnComponentHit(CapsuleComponent)
  (params (HitComponent :type Primitive%20Component%20Object%20Reference) (OtherActor :type Actor%20Object%20Reference) (OtherComp :type Primitive%20Component%20Object%20Reference) (NormalImpulse :type Vector :default "0, 0, 0") (Hit :type Hit%20Result%20Structure%20%28by%20ref%29))
  (Utilities|Casting|CastTo OtherActor)
  ;[0.06771 0.06771 0.06771] Создать Систему частиц
  (bind _output_get (Variables|Default|SetHP (- (Variables|Default|GetHP) 10)))
  (if (<= _output_get 0)
    (Physics|SetSimulatePhysics (Variables|Collision|GetCapsuleComponent) true)
    (Utilities|FlowControl|Delay 3.0)
    (Actor|DestroyActor)))

(event EventBeginPlay)

(event Collision|EventActorBeginOverlap
  (params (OtherActor :type Actor%20Object%20Reference)))

(event EventTick
  (params (DeltaSeconds :type Float%20%28single-precision%29))
  (Development|PrintString (Utilities|String|BuildString(Integer) "" "EnemyHP: " (Variables|Default|GetHP)) true true "(R=0.000000,G=0.660000,B=1.000000,A=1.000000)" 0.0))

(fn ConstructionScript)

(fn SetSpeed
  (params (Speed :type Float%20%28single-precision%29))
  (Variables|/Script/Engine.CharacterMovementComponent|SetMaxWalkSpeed (Variables|Character|GetCharacterMovement) (* Speed (Variables|Default|GetDefaultSpeed))))