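; AI controller Blueprint that runs a behavior tree and tracks a perceived target for an enemy.
; It starts the behavior tree on possess.
; AI Perception updates pass through a cast, then set the Player key in the enemy Blackboard to the sensed actor, or clear it when sensing fails.
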(event OnTargetPerceptionUpdated(AIPerception)
  (params (Actor :type Actor%20Object%20Reference) (Stimulus :type AI%20Stimulus%20Structure))
  (bind _asbp_player_character (Utilities|Casting|CastTo Actor))
  (if (.bSuccessfullySensed (Utilities|Struct|BreakAIStimulus Stimulus))
    (AI|Components|Blackboard|SetValueasObject (Variables|Default|GetEnemyBlackboard) (Variables|Default|GetPlayer) _asbp_player_character)
    (else
      (AI|Components|Blackboard|SetValueasObject (Variables|Default|GetEnemyBlackboard) (Variables|Default|GetPlayer) 0))))

(event EventPossess
  (params (PossessedPawn :type Pawn%20Object%20Reference))
  (AI|RunBehaviorTree))

(fn ConstructionScript)